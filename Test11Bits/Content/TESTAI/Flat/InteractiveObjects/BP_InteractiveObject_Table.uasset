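; BP_InteractiveObject_Table is a table interactive object whose usable spots come from four child actors.
; On BeginPlay, after the parent logic, it casts each child actor to BP_Spot_InteractiveObj and adds it uniquely to Spots.
; It then passes that array to InitSpotsStateMap to initialize spot state tracking.
; The construction script only calls the parent.
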(event EventBeginPlay
  (bind _spots (Variables|Default|GetSpots))
  (|CallParentFunction)
  (for _array_element (Utilities|Array|MakeArray (Variables|/Script/Engine.ChildActorComponent|GetChildActor (Variables|Default|GetChildActor1)) (Variables|/Script/Engine.ChildActorComponent|GetChildActor (Variables|Default|GetChildActor2)) (Variables|/Script/Engine.ChildActorComponent|GetChildActor (Variables|Default|GetChildActor3)) (Variables|/Script/Engine.ChildActorComponent|GetChildActor (Variables|Default|GetChildActor)))
    (bind _asbp_spot_interactive_obj (Utilities|Casting|CastToBP_Spot_InteractiveObj _array_element))
    (Utilities|Array|AddUnique _spots _asbp_spot_interactive_obj))
  (Class|InteractiveObject|InitSpotsStateMap _spots))

(fn ConstructionScript
  (|CallParentFunction))